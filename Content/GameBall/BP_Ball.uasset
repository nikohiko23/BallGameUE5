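; BP_Ball is a physics ball that moves at constant speed in the XY plane and destroys BP_Kegla pins it hits.
; BeginPlay launches MainSphere with a velocity-change impulse.
; Each tick rebuilds its linear velocity from the normalized X and Y components times Speed, dropping vertical motion, with DeltaSeconds wired as the normalization tolerance.
; MainSphere's hit event casts the other actor to BP_Kegla and destroys it.
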(event `self.ReceiveBeginPlay`
  ;[1 0.3462 0.9929] Начальное ускорение
  (`PrimitiveComponent.AddImpulse` (`self.MainSphere`) (`self.Impulse`) "None" true))

(event `self.ReceiveTick`
  (params (DeltaSeconds :type "Float (single-precision)"))
  (bind (_returnvalue_x _returnvalue_y) (`KismetMathLibrary.BreakVector` (`self.GetVelocity`)))
  ;[0.4553 0.427 1] Скорость мяча только в (x) и (y)
  (`PrimitiveComponent.SetPhysicsLinearVelocity` (`self.MainSphere`) (* (`KismetMathLibrary.Normal` (`KismetMathLibrary.MakeVector` _returnvalue_x _returnvalue_y) DeltaSeconds) (`self.Speed`)) false "None"))

(event `self.MainSphere.OnComponentHit`
  (params (HitComponent :type "PrimitiveComponent Object Reference") (OtherActor :type "Actor Object Reference") (OtherComp :type "PrimitiveComponent Object Reference") (NormalImpulse :type "Vector Structure") (Hit :type "HitResult Structure (by ref)"))
  ;[0.8591 1 0.4162] Разрушение обьекта кегли
  (bind _asbp_kegla (cast `/Game/GameBall/BP_Kegla` OtherActor))
  (`self.K2_DestroyActor` _asbp_kegla))

(fn `UserConstructionScript`)